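; Base weapon actor that takes shoot and reload input directly from player 0.
; Shooting sphere-traces forward from the camera and sends damage through BPI_HealthSystem to hit actors that implement it.
; Other hits and misses draw a debug sphere at the trace's impact point, sized by damage and lasting the reload duration.
; Reloading only hides the magazine mesh for the reload duration, with no ammo tracking or fire lockout.
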(event `EnhancedInput|/Game/Blueprints/Player/Input/Actions/IA_Shoot`
  (params (ActionValue :type Boolean) (ElapsedSeconds :type "Float (double-precision)") (TriggeredSeconds :type "Float (double-precision)") (InputAction :type "InputAction Object Reference" :default "/Game/Blueprints/Player/Input/Actions/IA_Shoot.IA_Shoot"))
  (:`Started`
    (`self.ShootWeapon`)))

(event `EnhancedInput|/Game/Blueprints/Player/Input/Actions/IA_Reload`
  (params (ActionValue :type Boolean) (ElapsedSeconds :type "Float (double-precision)") (TriggeredSeconds :type "Float (double-precision)") (InputAction :type "InputAction Object Reference" :default "/Game/Blueprints/Player/Input/Actions/IA_Reload.IA_Reload"))
  (:`Started`
    (`self.ReloadWeapon`)))

(event `self.ReceiveBeginPlay`
  (`self.EnableInput` (`GameplayStatics.GetPlayerController` 0)))

(event `/Game/Blueprints/Interfaces/BPI_WeaponSystem.ShootWeapon`
  (bind _transformcomponent (`PlayerCameraManager.TransformComponent` (`GameplayStatics.GetPlayerCameraManager` 0)))
  (bind _returnvalue (`SceneComponent.K2_GetComponentLocation` _transformcomponent))
  (bind (_outhit _returnvalue_2) (`KismetSystemLibrary.SphereTraceSingle` _returnvalue (+ _returnvalue (* (`SceneComponent.GetForwardVector` _transformcomponent) 4096.0)) 4.0 "TraceTypeQuery1"))
  (if _returnvalue_2
    (bind (_bblockinghit _binitialoverlap _time _distance _location _impactpoint _normal _impactnormal _physmat _hitactor) (`GameplayStatics.BreakHitResult` _outhit))
    (if (`KismetSystemLibrary.DoesImplementInterface` _hitactor "/Game/Blueprints/Interfaces/BPI_HealthSystem.BPI_HealthSystem_C")
      (message `/Game/Blueprints/Interfaces/BPI_HealthSystem.AdjustHealth` _hitactor true (`self.DamageAmount`))
      (else
        (`KismetSystemLibrary.DrawDebugSphere` _impactpoint (`self.DamageAmount`) 8 (struct :`R` 1.0 :`A` 1.0) (`self.ReloadDuration`) 1.0 :!label _label)))
    (else
      (goto _label))))

(event `/Game/Blueprints/Interfaces/BPI_WeaponSystem.ReloadWeapon`
  (`SceneComponent.SetVisibility` (`self.SM_Mag`) false false)
  (`KismetSystemLibrary.Delay` (`self.ReloadDuration`))
  (`SceneComponent.SetVisibility` (`self.SM_Mag`) true false))

(fn `UserConstructionScript`)