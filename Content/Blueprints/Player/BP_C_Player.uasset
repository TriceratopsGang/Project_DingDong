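; First-person player character with Enhanced Input movement, an air-only dash, ground pound, timeline-driven FOV zoom and pause toggle.
; Dash and ground pound use LaunchCharacter, with dash recharging after a delay on landing.
; Clamped health changes, triggered here by debug keys, route through SetPlayerHealth, which broadcasts updates.
; Shoot and reload handlers message the child-actor weapon through BPI_WeaponSystem, but their input events are unwired.
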(event EventBeginPlay
  (Input|AddInputMapping "/Game/Blueprints/Player/Input/IMC_Default.IMC_Default")
  (Character|InitPlayer))

(event EventOnLanded
  (params (Hit :type Hit%20Result%20Structure%20%28by%20ref%29))
  (Utilities|FlowControl|Delay (Variables|Character|Movement|GetDashCooldown)) ; Can replace this with a timer at the dash code
  (Variables|Character|Movement|SetbCanDash true)
  (Default|CallOnDashRefreshed))

(event Input|EnhancedActionEvents|EnhancedInputActionIA_Look
  (params (ActionValue :type Vector%202D%20Structure) (ElapsedSeconds :type Float%20%28double-precision%29) (TriggeredSeconds :type Float%20%28double-precision%29) (InputAction :type Input%20Action%20Object%20Reference :default "/Game/Blueprints/Player/Input/Actions/IA_Look.IA_Look"))
  (Input|HandleLook ActionValue))

(event Input|EnhancedActionEvents|EnhancedInputActionIA_Move
  (params (ActionValue :type Vector%202D%20Structure) (ElapsedSeconds :type Float%20%28double-precision%29) (TriggeredSeconds :type Float%20%28double-precision%29) (InputAction :type Input%20Action%20Object%20Reference :default "/Game/Blueprints/Player/Input/Actions/IA_Move.IA_Move"))
  (Input|HandleMove ActionValue))

(event Input|EnhancedActionEvents|EnhancedInputActionIA_Jump
  (params (ActionValue :type Boolean) (ElapsedSeconds :type Float%20%28double-precision%29) (TriggeredSeconds :type Float%20%28double-precision%29) (InputAction :type Input%20Action%20Object%20Reference :default "/Game/Blueprints/Player/Input/Actions/IA_Jump.IA_Jump"))
  (:Started
    (Character|Jump))
  (:Canceled
    (Character|StopJumping :!label _label))
  (:Completed
    (goto _label)))

(event Input|EnhancedActionEvents|EnhancedInputActionIA_Dash
  (params (ActionValue :type Boolean) (ElapsedSeconds :type Float%20%28double-precision%29) (TriggeredSeconds :type Float%20%28double-precision%29) (InputAction :type Input%20Action%20Object%20Reference :default "/Game/Blueprints/Player/Input/Actions/IA_Dash.IA_Dash"))
  (:Started
    (Input|HandleDash)))

(event Input|EnhancedActionEvents|EnhancedInputActionIA_GroundPound
  (params (ActionValue :type Boolean) (ElapsedSeconds :type Float%20%28double-precision%29) (TriggeredSeconds :type Float%20%28double-precision%29) (InputAction :type Input%20Action%20Object%20Reference :default "/Game/Blueprints/Player/Input/Actions/IA_GroundPound.IA_GroundPound"))
  (:Started
    (Input|HandleGroundPound)))

(event Input|EnhancedActionEvents|EnhancedInputActionIA_Pause
  (params (ActionValue :type Boolean) (ElapsedSeconds :type Float%20%28double-precision%29) (TriggeredSeconds :type Float%20%28double-precision%29) (InputAction :type Input%20Action%20Object%20Reference :default "/Game/Blueprints/Player/Input/Actions/IA_Pause.IA_Pause"))
  (:Started
    (Input|HandlePause)))

(event Input|EnhancedActionEvents|EnhancedInputActionIA_Shoot
  (params (ActionValue :type Boolean) (ElapsedSeconds :type Float%20%28double-precision%29) (TriggeredSeconds :type Float%20%28double-precision%29) (InputAction :type Input%20Action%20Object%20Reference :default "/Game/Blueprints/Player/Input/Actions/IA_Shoot.IA_Shoot"))
  ;[0.005182 0.005182 0.005182] IDK if this should be here or in the weapon
)

(event Input|EnhancedActionEvents|EnhancedInputActionIA_Zoom
  (params (ActionValue :type Boolean) (ElapsedSeconds :type Float%20%28double-precision%29) (TriggeredSeconds :type Float%20%28double-precision%29) (InputAction :type Input%20Action%20Object%20Reference :default "/Game/Blueprints/Player/Input/Actions/IA_Zoom.IA_Zoom"))
  (:Started
    (bind _alpha (Timeline|TL_Zoom Play)
      (:Update
        (Input|HandleZoom _alpha))))
  (:Canceled
    (Timeline|TL_Zoom Reverse))
  (:Completed
    (Timeline|TL_Zoom Reverse)))

(event Input|EnhancedActionEvents|EnhancedInputActionIA_Reload
  (params (ActionValue :type Boolean) (ElapsedSeconds :type Float%20%28double-precision%29) (TriggeredSeconds :type Float%20%28double-precision%29) (InputAction :type Input%20Action%20Object%20Reference :default "/Game/Blueprints/Player/Input/Actions/IA_Reload.IA_Reload"))
  ;[0.005182 0.005182 0.005182] IDK if this should be here or in the weapon
)

(event Input|KeyboardEvents|DebugKeyPageDown
  (params (Key :type Key%20Structure) (ActionValue :type Input%20Action%20Value%20Structure))
  (:Pressed
    (CallFunction|AdjustHealth true 1e+01)))

(event Input|KeyboardEvents|DebugKeyPageUp
  (params (Key :type Key%20Structure) (ActionValue :type Input%20Action%20Value%20Structure))
  (:Pressed
    (CallFunction|AdjustHealth false 1e+01)))

(fn ConstructionScript)

(fn AddInputMapping
  (params (MappingContext :type Input%20Mapping%20Context%20Object%20Reference))
  (bind _asplayer_controller (Utilities|Casting|CastToPlayerController (Pawn|GetController)))
  (Utilities|IsValid (PlayerController|LocalPlayerSubsystems|GetEnhancedInputLocalPlayerSubsystem _asplayer_controller)
    (:Is%20Valid
      (Input|AddMappingContext (PlayerController|LocalPlayerSubsystems|GetEnhancedInputLocalPlayerSubsystem _asplayer_controller) MappingContext 0 "(bIgnoreAllPressedKeysUntilRelease=True,bForceImmediately=False,bNotifyUserSettings=False)"))
    (:Is%20Not%20Valid
      (Development|PrintString "\"AddInputMapping\" FAILED" true true "(R=1.000000,G=0.000000,B=0.000000,A=1.000000)" 3.0))))

(fn HandleLook
  (params (InVec :type Vector%202D%20Structure))
  (Pawn|Input|AddControllerYawInput (.x InVec))
  (Pawn|Input|AddControllerPitchInput (.y InVec)))

(fn HandleMove
  (params (InVec :type Vector%202D%20Structure))
  (Pawn|Input|AddMovementInput (Transformation|GetActorRightVector) (.x InVec) false)
  (Pawn|Input|AddMovementInput (Transformation|GetActorForwardVector) (.y InVec) false))

(fn SetPlayerHealth
  (params (Type :type String) (NewCurrent :type Float%20%28double-precision%29) (NewMax :type Float%20%28double-precision%29))
  (switch string Type
    (:Current
      (Variables|Character|Vitals|SetHealthCurrent NewCurrent)
      (Default|CallOnHealthUpdated (Variables|Character|Vitals|GetHealthCurrent) (Variables|Character|Vitals|GetHealthMax)))
    (:Max
      (Variables|Character|Vitals|SetHealthMax NewMax)
      (Default|CallOnHealthUpdated (Variables|Character|Vitals|GetHealthCurrent) (Variables|Character|Vitals|GetHealthMax)))
    (:Both
      (Variables|Character|Vitals|SetHealthMax NewMax)
      (Variables|Character|Vitals|SetHealthCurrent NewCurrent)
      (Default|CallOnHealthUpdated (Variables|Character|Vitals|GetHealthCurrent) (Variables|Character|Vitals|GetHealthMax)))))

(fn InitPlayer
  (Character|Vitals|SetPlayerHealth "Both" 1e+02 1e+02)
  (bind _output_get (Variables|Character|Camera|SetFOVBase (Variables|/Script/Engine.CameraComponent|GetFieldOfView (Variables|Default|GetFPSCamera))))
  (Variables|Character|Camera|SetFOVZoom (/ _output_get 2.0)))

(fn HandleDash
  (bind _returnvalue (Transformation|GetVelocity))
  (if (and (Variables|Character|Movement|GetbCanDash) (AI|Components|NavMovement|IsFalling (Variables|Character|GetCharacterMovement)))
    (Character|LaunchCharacter (* (Math|Vector|MakeVector (.x _returnvalue) (.y _returnvalue) 0.0) (Variables|Character|Movement|GetDashPower)) false false)
    (Variables|Character|Movement|SetbCanDash false)
    (Default|CallOnDashed)
    (else
      (Audio|PlaySound2D "/Engine/EditorSounds/Notifications/CompileFailed_Cue.CompileFailed_Cue" 0.2 1.0 0.0 0 0))))

(fn HandleGroundPound
  (if (AI|Components|NavMovement|IsFalling (Variables|Character|GetCharacterMovement))
    (Character|LaunchCharacter (* (Transformation|GetActorUpVector) (* (Variables|Character|Movement|GetGroundPoundPower) -1.0)) false false)
    (Default|CallOnGroundPound)))

(fn HandlePause
  (Game|SetGamePaused (not (Game|IsGamePaused))))

(fn HandleShoot
  (bind _childactor (Variables|/Script/Engine.ChildActorComponent|GetChildActor (Variables|Default|GetActiveWeapon))
    (:then
      (if (Utilities|DoesObjectImplementInterface _childactor "/Game/Blueprints/Interfaces/BPI_WeaponSystem.BPI_WeaponSystem_C")
        (Class|BPIWeaponSystem|ShootWeapon(Message) _childactor)))
    (:else)))

(fn HandleZoom
  (params (Alpha :type Float%20%28single-precision%29))
  (Camera|SetFieldOfView (Variables|Default|GetFPSCamera) (Math|Float|MapRangeClamped Alpha 0.0 1.0 (Variables|Character|Camera|GetFOVBase) (Variables|Character|Camera|GetFOVZoom))))

(fn HandleReload
  (bind _childactor (Variables|/Script/Engine.ChildActorComponent|GetChildActor (Variables|Default|GetActiveWeapon))
    (:then
      (if (Utilities|DoesObjectImplementInterface _childactor "/Game/Blueprints/Interfaces/BPI_WeaponSystem.BPI_WeaponSystem_C")
        (Class|BPIWeaponSystem|ReloadWeapon(Message) _childactor)))
    (:else)))

(fn AdjustHealth
  (params (bIsDamage :type Boolean) (AdjustmentAmount :type Float%20%28double-precision%29))
  (if (> AdjustmentAmount 0.0)
    (if bIsDamage
      (Character|Vitals|SetPlayerHealth "Current" (Math|Float|Clamp(Float) (- (Variables|Character|Vitals|GetHealthCurrent) AdjustmentAmount) 0.0 (Variables|Character|Vitals|GetHealthMax)) 0.0)
      (return (Variables|Character|Vitals|GetHealthCurrent))
      (else
        (Character|Vitals|SetPlayerHealth "Current" (Math|Float|Clamp(Float) (+ (Variables|Character|Vitals|GetHealthCurrent) AdjustmentAmount) 0.0 (Variables|Character|Vitals|GetHealthMax)) 0.0)
        (return (Variables|Character|Vitals|GetHealthCurrent))))))

(fn GetHealth
  (return (Variables|Character|Vitals|GetHealthCurrent) (Variables|Character|Vitals|GetHealthMax)))

(fn GetHealthPercentage
  (return (/ (Variables|Character|Vitals|GetHealthCurrent) (Variables|Character|Vitals|GetHealthMax))))